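; BP_Villager is a villager character that walks to resource tiles or back to camp using AIMoveTo.
; Move_To_Tile heads for a resource actor and, on success, tells it to show a villager, then destroys itself.
; Move_To_Camp sends it to a hard-coded camp strip with a random Y offset.
; A behavior tree launch is present but never runs.
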(event `self.ReceiveBeginPlay`)

(event `Move_To_Tile`
  (params (Ressource_Actor :type "/Game/Indian/Actors/Ressources/BP_Ressources_Actor Object Reference"))
  (`|AIMoveTo` (`PawnMovementComponent.GetPawnOwner` (`self.CharacterMovement`)) (`self.K2_GetActorLocation` Ressource_Actor) null 500.0
    (:`OnSuccess`
      (`/Game/Indian/Actors/Ressources/BP_Ressources_Actor.Show_Villager` Ressource_Actor)
      (`self.K2_DestroyActor`))))

(event `Move_To_Camp`
  (`|AIMoveTo` (`PawnMovementComponent.GetPawnOwner` (`self.CharacterMovement`)) (`KismetMathLibrary.MakeVector` -500.0 (`KismetMathLibrary.RandomFloatInRange` -1000.0 1000.0) 230.0) null 100.0))

(fn `UserConstructionScript`)