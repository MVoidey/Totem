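; BP_Ressource_To_Place_Actor is a clickable marker for a spot where the player can place a new resource.
; On BeginPlay it creates a dynamic instance of Ressource_To_Place_Mat on its mesh, tints it with its Color variable and caches the BP_TopDownCharacter player.
; When clicked, it passes its own location to the player's PlaceNewRessource function.
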(event `self.ReceiveBeginPlay`
  (bind _returnvalue (`PrimitiveComponent.CreateDynamicMaterialInstance` (`self.Ressource_Mesh`) 0 "/Game/Indian/Material/Ressources/Ressource_To_Place_Mat.Ressource_To_Place_Mat" "None"))
  (`MaterialInstanceDynamic.SetVectorParameterValue` _returnvalue "Color" (`self.Color`))
  (bind _astop_down_character (cast `/Game/TopDownBP/Blueprints/BP_TopDownCharacter` (`GameplayStatics.GetPlayerCharacter` 0)))
  (set `self.Player` _astop_down_character))

(event `self.ReceiveActorOnClicked`
  (params (ButtonPressed :type "Key Structure"))
  (`/Game/TopDownBP/Blueprints/BP_TopDownCharacter.Place_New_Ressource` (`self.Player`) (`self.K2_GetActorLocation`)))

(fn `UserConstructionScript`)