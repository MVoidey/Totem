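; BP_Ressources_Actor is a clickable resource tile that villagers harvest for the player, destroying itself once depleted.
; A looping timer moves an amount equal to the assigned villager count into the player's stock and refreshes the HUD.
; Add/Remove events update player villager counts, with visible villager slots and spawned BP_Villagers walking back to camp on removal or depletion.
; Clicking toggles its Ressource_Widget, hiding other tiles' widgets; hover handlers are empty.
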(event `self.ReceiveBeginPlay`
  ;[1 1 1] Création Player_Ref
  (bind _astop_down_character (cast `/Game/TopDownBP/Blueprints/BP_TopDownCharacter` (`GameplayStatics.GetPlayerCharacter` 0)))
  (set `self.Player_Ref` _astop_down_character)
  ;[1 0.2552 0.2552] Création du timer pour donner les ressources au joueur
  (bind _returnvalue (`KismetSystemLibrary.K2_SetTimer` null "Give_Ressources_to_Player" (`self.Timer_Value`) true))
  (set `self.Timer` _returnvalue)
  (`self.Set_Type` "NewEnumerator0")
  ;[1 1 1] Bind les event pour afficher/cacher l'outline
  (add `self.OnBeginCursorOver` (delegate `On_Mouse_Hover`))
  (add `self.OnEndCursorOver` (delegate `On_Mouse_Hover_End`))
  (`KismetSystemLibrary.Delay` 0.2)
  (`self.Set_Widget`))

(event `On_Mouse_Hover` :!signature `self.OnBeginCursorOver`
  (params (TouchedActor :type "Actor Object Reference"))
  ;[1 1 1] Bind les event pour afficher/cacher l'outline
)

(event `On_Mouse_Hover_End` :!signature `self.OnEndCursorOver`
  (params (TouchedActor :type "Actor Object Reference"))
  ;[1 1 1] Bind les event pour afficher/cacher l'outline
)

(event `Set_Widget`
  (bind _asressource_widget (cast `/Game/Indian/HUD/Ressources_Widget/Ressource_Widget` (`WidgetComponent.GetWidget` (`self.Ressource_Widget`))))
  (`/Game/Indian/HUD/Ressources_Widget/Ressource_Widget.Set_Owner` _asressource_widget self))

(event `Set_Type`
  (params (Tile_Type :type "/Game/Indian/Utilities/Ressource_Type Enum" :default "NewEnumerator0"))
  (set `self.Tile_Type` Tile_Type))

(event `self.ReceiveActorOnClicked`
  (params (ButtonPressed :type "Key Structure"))
  ;[1 1 1] On Clicked Event pour afficher le Ressource_Widget
  (if (`SceneComponent.bVisible` (`self.Ressource_Widget`))
    (`SceneComponent.SetVisibility` (`self.Ressource_Widget`) false false)
    (else
      (bind _outactors (`GameplayStatics.GetAllActorsOfClass` "BP_Ressources_Actor_C"))
      (for _array_element _outactors
        (`SceneComponent.SetVisibility` (`/Game/Indian/Actors/Ressources/BP_Ressources_Actor.Ressource_Widget` _array_element) false false))
      (`SceneComponent.SetVisibility` (`self.Ressource_Widget`) true false))))

(event `Add_Villager`
  (bind _player_ref (`self.Player_Ref`))
  (bind _tile_type (`self.Tile_Type`))
  (bind _villager_repartition (`/Game/TopDownBP/Blueprints/BP_TopDownCharacter.Villager_Repartition` _player_ref))
  ;[1 1 1] Add_Villager
  (if (< (`self.Villager_Amount`) (`self.Max_Villager`))
    (if (> (`/Game/TopDownBP/Blueprints/BP_TopDownCharacter.Villager_Available` (`self.Player_Ref`)) 0)
      (`/Engine/EditorBlueprintResources/StandardMacros.DecrementInt` (`/Game/TopDownBP/Blueprints/BP_TopDownCharacter.Villager_Available` _player_ref)
        (:`  `
          (`/Engine/EditorBlueprintResources/StandardMacros.IncrementInt` (`self.Villager_Amount`)
            (:`  `
              (`BlueprintMapLibrary.Map_Add` _villager_repartition _tile_type (+ (`BlueprintMapLibrary.Map_Find` _villager_repartition _tile_type) 1))
              (`/Game/TopDownBP/Blueprints/BP_TopDownCharacter.Send_Villager_To Tile` (`self.Player_Ref`) self))))))))

(event `Remove_Villager`
  (bind _tile_type (`self.Tile_Type`))
  (bind _player_ref (`self.Player_Ref`))
  (bind _villager_repartition (`/Game/TopDownBP/Blueprints/BP_TopDownCharacter.Villager_Repartition` _player_ref))
  ;[1 1 1] Remove_Villager
  (if (> (`self.Villager_Amount`) 0)
    (`/Engine/EditorBlueprintResources/StandardMacros.DecrementInt` (`self.Villager_Amount`)
      (:`  `
        (`/Engine/EditorBlueprintResources/StandardMacros.IncrementInt` (`/Game/TopDownBP/Blueprints/BP_TopDownCharacter.Villager_Available` _player_ref)
          (:`  `
            (`BlueprintMapLibrary.Map_Add` _villager_repartition _tile_type (- (`BlueprintMapLibrary.Map_Find` _villager_repartition _tile_type) 1))
            (`self.Hide_Villager`)))))))

(event `Show_Villager`
  ;[1 1 1] Show_Villager
  (`SceneComponent.SetVisibility` (`|GetArrayItem` (`|MakeArray` (`self.Villager1`) (`self.Villager2`) (`self.Villager3`) (`self.Villager4`) (`self.Villager5`)) (`self.Villager_Visible`)) true false)
  (`/Engine/EditorBlueprintResources/StandardMacros.IncrementInt` (`self.Villager_Visible`)))

(event `Hide_Villager`
  (bind (_returnvalue_x _returnvalue_y) (`KismetMathLibrary.BreakVector` (`self.K2_GetActorLocation`)))
  (bind _villager_visible (`self.Villager_Visible`))
  ;[1 1 1] Hide_Villager
  (`/Engine/EditorBlueprintResources/StandardMacros.DecrementInt` _villager_visible
    (:`  `
      (`SceneComponent.SetVisibility` (`|GetArrayItem` (`|MakeArray` (`self.Villager1`) (`self.Villager2`) (`self.Villager3`) (`self.Villager4`) (`self.Villager5`)) _villager_visible) false false)
      (bind _returnvalue (`|SpawnActorFromClass` "/Game/Indian/Actors/Villager/BP_Villager.BP_Villager_C" (`KismetMathLibrary.MakeTransform` (`KismetMathLibrary.MakeVector` (- _returnvalue_x 600.0) _returnvalue_y 230.0)) "Undefined" "OverrideRootScale" null null))
      (`/Game/Indian/Actors/Villager/BP_Villager.Move_To_Camp` _returnvalue)
      (`KismetArrayLibrary.Array_Add` (`/Game/TopDownBP/Blueprints/BP_TopDownCharacter.Villagers_Actor_List` (`self.Player_Ref`)) _returnvalue))))

(event `Give_Ressources_to_Player`
  (bind _tile_type (`self.Tile_Type`))
  (bind _returnvalue (- (`self.Ressource_Amount`) (`self.Villager_Amount`)))
  (bind _main_hud (`/Game/TopDownBP/Blueprints/BP_TopDownCharacter.Main_HUD` (`self.Player_Ref`)))
  (bind _ressources_stock (`/Game/TopDownBP/Blueprints/BP_TopDownCharacter.Ressources_Stock` (`self.Player_Ref`)))
  (bind _value (`BlueprintMapLibrary.Map_Find` _ressources_stock _tile_type))
  ;[1 1 1] Give Ressource to Player
  (if (<= _returnvalue 0)
    (`BlueprintMapLibrary.Map_Add` _ressources_stock _tile_type (+ (`self.Ressource_Amount`) _value))
    (`/Game/Indian/HUD/Main_HUD/Main_HUD.Update_Ressources` _main_hud)
    (`self.Destroy_When_Empty`)
    (else
      (set `self.Ressource_Amount` _returnvalue)
      (`BlueprintMapLibrary.Map_Add` _ressources_stock _tile_type (+ _value (* (`self.Villager_Amount`) 1)))
      (`/Game/Indian/HUD/Main_HUD/Main_HUD.Update_Ressources` _main_hud))))

(event `Destroy_When_Empty`
  ;[1 1 1] Destroy Actor when Empty
  (`/Game/Indian/Utilities/BP_Custom_Macro.For_Loop_With_Delay` 0 (- (`self.Villager_Amount`) 1) 0.2
    (:`Loop_Body`
      (`self.Hide_Villager`)
      (`/Engine/EditorBlueprintResources/StandardMacros.IncrementInt` (`/Game/TopDownBP/Blueprints/BP_TopDownCharacter.Villager_Available` (`self.Player_Ref`))))
    (:`Completed`
      (`self.K2_DestroyActor`))))

(fn `UserConstructionScript`)