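; Map tile actor that serves as a placement spot for new buildings.
; Cursor hover passes the tile's location to the cached BP_TopDownCharacter, and a click ends placement mode and spawns the pending BP_Buildings_Actor.
; Random radial scattering of grass, mushroom and other decorative meshes exists in the construction script but is disconnected, as is an alternative PlaceNewRessource placement path.
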(event `self.ReceiveBeginPlay`
  (bind _astop_down_character (cast `/Game/TopDownBP/Blueprints/BP_TopDownCharacter` (`GameplayStatics.GetPlayerCharacter` 0)))
  (set `self.Player` _astop_down_character))

(event `self.ReceiveActorBeginCursorOver`
  (`/Game/TopDownBP/Blueprints/BP_TopDownCharacter.Set_New_Item_Location` (`self.Player`) (`self.K2_GetActorLocation`)))

(event `self.ReceiveActorOnClicked`
  (params (ButtonPressed :type "Key Structure"))
  (bind _player (`self.Player`))
  (set `/Game/TopDownBP/Blueprints/BP_TopDownCharacter.Is_Placing_New_Item?` false _player)
  (bind _asbuildings_actor (cast `/Game/Indian/Actors/Buildings/BP_Buildings_Actor` (`/Game/TopDownBP/Blueprints/BP_TopDownCharacter.New_Item_Actor` _player)))
  (`/Game/Indian/Actors/Buildings/BP_Buildings_Actor.Spawn` _asbuildings_actor))

(fn `UserConstructionScript`)