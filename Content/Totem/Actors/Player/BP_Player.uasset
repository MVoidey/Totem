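; Player Blueprint for an island tile game that manages HUDs, villagers and placement of new resources.
; BeginPlay creates the in-game and hidden tile-choice widgets, reads occupied locations from BP_Island_Generator and spawns a row of villagers.
; Send_Villager_ToTile dispatches and delists the first villager.
; A preview actor follows free locations and hides on occupied ones; placement spawns the mapped resource class, destroys the preview and records the location.
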(event `self.ReceiveBeginPlay`
  (`|ExecutionSequence`
    (:`then_0`
      ;[1 1 1] Create Main HUD
      (bind _returnvalue (`|CreateWidget` "/Game/Totem/HUD/InGame_Widget/WBP_InGame.WBP_InGame_C"))
      (bind _output_get (set `self.WBP_InGame` _returnvalue))
      (`UserWidget.AddToViewport` _output_get 0)
      ;[1 1 1] Create Tile Choice HUD
      (bind _returnvalue_2 (`|CreateWidget` "/Game/Totem/HUD/Tile_Choice_Widget/WBP_Tile_Choice.WBP_Tile_Choice_C"))
      (bind _output_get_2 (set `self.Tile_Choice_HUD` _returnvalue_2))
      (`UserWidget.AddToViewport` _output_get_2 0)
      (`Widget.SetVisibility` _output_get_2 "Hidden")
      ;[1 1 1] Set les positions indisponible pour de nouveaux items
      (bind _returnvalue_3 (`GameplayStatics.GetActorOfClass` "/Game/Totem/Actors/Grid_Manager/BP_Island_Generator.BP_Island_Generator_C"))
      (set `self.Non_Available_Locations` (`/Game/Totem/Actors/Grid_Manager/BP_Island_Generator.Occupied_Locations` _returnvalue_3)))
    (:`then_1`
      (for _index (range 1 (+ (`self.Villager_Amount`) 1))
        (bind _returnvalue_4 (`|SpawnActorFromClass` "/Game/Totem/Actors/Villager/BP_Villager.BP_Villager_C" (`KismetMathLibrary.MakeTransform` (`KismetMathLibrary.MakeVector` -1000.0 (* _index 100.0) 230.0) (`KismetMathLibrary.MakeRotator` 0.0 0.0 (`KismetMathLibrary.RandomFloatInRange` 0.0 360.0))) "Undefined" "OverrideRootScale" null null))
        (`KismetArrayLibrary.Array_Add` (`self.Villagers_Actor_List`) _returnvalue_4)))))

(event `Send_Villager_To Tile`
  (params (Ressource_Actor :type "/Game/Totem/Actors/Interactable/Ressources/BP_Ressources_Actor Object Reference"))
  (bind _villagers_actor_list (`self.Villagers_Actor_List`))
  ;[1 1 1] Add/Remove Villager
  (`/Game/Totem/Actors/Villager/BP_Villager.Move_To_Tile` (`|GetArrayItem` _villagers_actor_list) Ressource_Actor)
  (`KismetArrayLibrary.Array_Remove` _villagers_actor_list))

(event `Key|SpaceBar`
  (params (Key :type "Key Structure")))

(event `Place_New_Ressource`
  (params (Location :type "Vector Structure"))
  ;[1 1 1] Place New Ressource Actor
  (if (`self.Available_Location?`)
    (`|SpawnActorFromClass` (`BlueprintMapLibrary.Map_Find` (`self.Ressource_Class_Actor`) (`self.New_Ressource_Type`)) (`KismetMathLibrary.MakeTransform` (`KismetMathLibrary.MakeVector` (.x Location) (.y Location) 200.0)) "Undefined" "OverrideRootScale" null null)
    (`self.K2_DestroyActor` (`self.New_Item_Actor`))
    (set `self.Is_Placing_New_Item?` false)
    (`KismetArrayLibrary.Array_Add` (`self.Non_Available_Locations`) Location)))

(event `Set_New_Item_Location`
  (params (Location :type "Vector Structure"))
  (bind _new_item_actor (`self.New_Item_Actor`))
  ;[1 1 1] Set New Item Location
  (if (`self.Is_Placing_New_Item?`)
    (if (`KismetArrayLibrary.Array_Contains` (`self.Non_Available_Locations`) Location)
      (`self.SetActorHiddenInGame` _new_item_actor true)
      (set `self.Available_Location?` false)
      (else
        (`self.SetActorHiddenInGame` _new_item_actor false)
        (`self.K2_SetActorLocation` _new_item_actor Location false false)
        (set `self.Available_Location?` true)))))

(fn `UserConstructionScript`)