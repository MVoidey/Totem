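; Player controller for a top-down building game that creates the HUD and tile choice widgets and handles camera, game speed and mouse interaction.
; The camera pawn pans by keys, screen edges or right-drag, while spring-arm zoom adjusts pitch and max speed.
; Speed hotkeys, with pause toggle, set CustomTimeDilation on all actors except camera and controller, syncing the time widget.
; Left-click traces place items, create building links, or select and deselect interactables.
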(event `self.ReceiveBeginPlay`
  (`|ExecutionSequence`
    (:`then_0`
      ;[1 1 1] Create Main HUD
      (bind _returnvalue (`|CreateWidget` "/Game/Totem/HUD/InGame_Widget/WBP_InGame.WBP_InGame_C"))
      (bind _output_get (set `self.WBP_InGame` _returnvalue))
      (`UserWidget.AddToViewport` _output_get 0))
    (:`then_1`
      ;[1 1 1] Create Tile Choice HUD
      (bind _returnvalue_2 (`|CreateWidget` "/Game/Totem/HUD/Tile_Choice_Widget/WBP_Tile_Choice.WBP_Tile_Choice_C"))
      (bind _output_get_2 (set `self.Tile_Choice_HUD` _returnvalue_2))
      (`UserWidget.AddToViewport` _output_get_2 0)
      (`Widget.SetVisibility` _output_get_2 "Hidden"))))

(event `InputAxisKey|MouseX`
  (params (AxisValue :type "Float (single-precision)"))
  (bind (_returnvalue_x _returnvalue_y) (`KismetMathLibrary.BreakVector2D` (`WidgetLayoutLibrary.GetViewportSize`)))
  (bind _bp_camera_player (`/Game/Totem/Utilities/Function_Lib/Totem_Function_Library.Cast_Camera_Player`))
  (bind _returnvalue (`self.GetActorRightVector` (`/Game/Totem/Utilities/Function_Lib/Totem_Function_Library.Cast_Camera_Player`)))
  (bind _returnvalue_2 (/ (`self.GetMousePosition` (`GameplayStatics.GetPlayerController` 0)) _returnvalue_x))
  ;[1 1 1] Deplace la camera si la sourirs est trop proche des bords
  (if (> _returnvalue_2 0.995)
    (`Pawn.AddMovementInput` _bp_camera_player _returnvalue 1.0 false)
    (elif (< _returnvalue_2 0.005)
      (`Pawn.AddMovementInput` _bp_camera_player _returnvalue -1.0 false))))

(event `InputAxis|MoveForward` :paused true
  (params (AxisValue :type "Float (single-precision)"))
  ;[1 1 1] Movement Input Clavier
  (`Pawn.AddMovementInput` (`/Game/Totem/Utilities/Function_Lib/Totem_Function_Library.Cast_Camera_Player`) (`self.GetActorForwardVector` (`/Game/Totem/Utilities/Function_Lib/Totem_Function_Library.Cast_Camera_Player`)) AxisValue false))

(event `InputAxisKey|MouseX`
  (params (AxisValue :type "Float (single-precision)"))
  (bind _bp_camera_player (`/Game/Totem/Utilities/Function_Lib/Totem_Function_Library.Cast_Camera_Player`))
  (bind (_returnvalue_x _returnvalue_y) (`KismetMathLibrary.BreakVector2D` (`WidgetLayoutLibrary.GetViewportSize`)))
  (bind _returnvalue (`self.GetActorForwardVector` (`/Game/Totem/Utilities/Function_Lib/Totem_Function_Library.Cast_Camera_Player`)))
  (bind _returnvalue_2 (/ (`.LocationY` (`self.GetMousePosition` (`GameplayStatics.GetPlayerController` 0))) _returnvalue_y))
  ;[1 1 1] Deplace la camera si la sourirs est trop proche des bords
  (if (> _returnvalue_2 0.995)
    (`Pawn.AddMovementInput` _bp_camera_player _returnvalue -1.0 false)
    (elif (< _returnvalue_2 0.005)
      (`Pawn.AddMovementInput` _bp_camera_player _returnvalue 1.0 false))))

(event `InputAxis|MoveRight` :paused true
  (params (AxisValue :type "Float (single-precision)"))
  ;[1 1 1] Movement Input Clavier
  (`Pawn.AddMovementInput` (`/Game/Totem/Utilities/Function_Lib/Totem_Function_Library.Cast_Camera_Player`) (`self.GetActorRightVector` (`/Game/Totem/Utilities/Function_Lib/Totem_Function_Library.Cast_Camera_Player`)) AxisValue false))

(event `InputAction|Mouse_Right_Click`
  (params (Key :type "Key Structure"))
  ;[1 1 1] Movement Input avec la Souris
  (:`Pressed`
    (if (`self.Placing_Link?`)
      (`/Game/Totem/HUD/Building_Widget/WBP_Building_Base.Mouse_Right_Click` (`/Game/Totem/Actors/Interactable/Buildings/BP_Buildings.WBP_Building_Base` (`self.Building_Placing_Link`)))
      (else
        (set `self.Right_Clicked?` true))))
  (:`Released`
    (set `self.Right_Clicked?` false)))

(event `InputAxis|MouseMoveForward` :paused true
  (params (AxisValue :type "Float (single-precision)"))
  ;[1 1 1] Movement Input avec la Souris
  (if (`self.Right_Clicked?`)
    (`Pawn.AddMovementInput` (`/Game/Totem/Utilities/Function_Lib/Totem_Function_Library.Cast_Camera_Player`) (`KismetMathLibrary.GetForwardVector` (`KismetMathLibrary.MakeRotator` 0.0 0.0 (.yaw (`self.GetControlRotation`)))) (* AxisValue (`self.Mouse_Move_Multiplier`)) false)))

(event `InputAxis|MouseMoveRight` :paused true
  (params (AxisValue :type "Float (single-precision)"))
  ;[1 1 1] Movement Input avec la Souris
  (if (`self.Right_Clicked?`)
    (`Pawn.AddMovementInput` (`/Game/Totem/Utilities/Function_Lib/Totem_Function_Library.Cast_Camera_Player`) (`KismetMathLibrary.GetRightVector` (`KismetMathLibrary.MakeRotator` 0.0 0.0 (.yaw (`self.GetControlRotation`)))) (* AxisValue (`self.Mouse_Move_Multiplier`)) false)))

(event `InputAction|Zoom In` :paused true
  (params (Key :type "Key Structure"))
  (bind _springarm (`/Game/Totem/Actors/Player/BP_Camera_Player.SpringArm` (`/Game/Totem/Utilities/Function_Lib/Totem_Function_Library.Cast_Camera_Player`)))
  (bind (_returnvalue_roll _returnvalue_pitch _returnvalue_yaw) (`KismetMathLibrary.BreakRotator` (`SpringArmComponent.GetTargetRotation` _springarm)))
  (bind _targetarmlength (`SpringArmComponent.TargetArmLength` _springarm))
  ;[1 1 1] Zoom In/Out
  (:`Pressed`
    (set `self.Zoom_Length_Speed` 1000.0)
    (set `self.Zoom_Rotation_Speed` 3.0)
    (if (> _targetarmlength 5000.0) :!label _label
      (set `SpringArmComponent.TargetArmLength` (- _targetarmlength (`self.Zoom_Length_Speed`)) _springarm)
      (`SceneComponent.K2_SetRelativeRotation` _springarm (`KismetMathLibrary.MakeRotator` _returnvalue_roll (+ _returnvalue_pitch (`self.Zoom_Rotation_Speed`)) _returnvalue_yaw) false false)
      (`/Engine/EditorBlueprintResources/StandardMacros.IncrementInt` (`self.Zoom_Level`)
        (:`  `
          (`self.Set_Player_Max_Speed` :!label _label_2))))))

(event `InputAxis|Trigger_zoom_In`
  (params (AxisValue :type "Float (single-precision)"))
  ;[1 1 1] Zoom In/Out
  (if (> AxisValue 0.0)
    (set `self.Zoom_Length_Speed` 200.0)
    (set `self.Zoom_Rotation_Speed` 0.6)
    (goto _label)))

(event `InputAction|Zoom Out` :paused true
  (params (Key :type "Key Structure"))
  (bind _springarm (`/Game/Totem/Actors/Player/BP_Camera_Player.SpringArm` (`/Game/Totem/Utilities/Function_Lib/Totem_Function_Library.Cast_Camera_Player`)))
  (bind (_returnvalue_roll _returnvalue_pitch _returnvalue_yaw) (`KismetMathLibrary.BreakRotator` (`SpringArmComponent.GetTargetRotation` _springarm)))
  (bind _targetarmlength (`SpringArmComponent.TargetArmLength` _springarm))
  ;[1 1 1] Zoom In/Out
  (:`Pressed`
    (if (< _targetarmlength 15000.0) :!label _label_3
      (set `SpringArmComponent.TargetArmLength` (+ _targetarmlength (`self.Zoom_Length_Speed`)) _springarm)
      (`SceneComponent.K2_SetRelativeRotation` _springarm (`KismetMathLibrary.MakeRotator` _returnvalue_roll (- _returnvalue_pitch (`self.Zoom_Rotation_Speed`)) _returnvalue_yaw) false false)
      (`/Engine/EditorBlueprintResources/StandardMacros.DecrementInt` (`self.Zoom_Level`)
        (:`  `
          (goto _label_2))))))

(event `InputAxis|Trigger_Zoom_Out`
  (params (AxisValue :type "Float (single-precision)"))
  ;[1 1 1] Zoom In/Out
  (if (> AxisValue 0.0)
    (set `self.Zoom_Length_Speed` 200.0)
    (set `self.Zoom_Rotation_Speed` 0.6)
    (goto _label_3)))

(event `InputAction|Speed_Control`
  (params (Key :type "Key Structure"))
  (bind _outmappings (`InputSettings.GetActionMappingByName` (`InputSettings.GetInputSettings`) "Speed_Control"))
  ;[1 1 1] Speed Control
  (:`Pressed`
    (if (not (`self.Is_Placing_New_Item?`))
      (if (not (and (== (`self.Current_Game_Speed`) 0) (== Key (`.Key` (break `InputActionKeyMapping` (`|GetArrayItem` _outmappings))))))
        (for (_array_element _array_index) _outmappings
          (if (== Key (`.Key` (break `InputActionKeyMapping` _array_element)))
            (`self.Set_Game_Speed` _array_index) ; On définie le nouveau Game Speed
            (bind _foundwidgets (`WidgetBlueprintLibrary.GetAllWidgetsOfClass` "/Game/Totem/HUD/InGame_Widget/WBP_InGame.WBP_InGame_C"))
            (`/Game/Totem/HUD/InGame_Widget/WBP_Time_Control.Set_Game_Speed_From_Player_Controller` (`/Game/Totem/HUD/InGame_Widget/WBP_InGame.WBP_Time_Control` (`|GetArrayItem` _foundwidgets)) _array_index) ; On modifie WBP_Time_Control
            (set `self.Current_Game_Speed` _array_index)))
        (else
          (bind _output_get (set `self.Current_Game_Speed` 1)) ; Cette suite de nodes permet au joueur\nde repasser en vitesse 1 si le jeu est déjà\nen vitesse 0, en rappuyant sur touche de\nvitesse 0. Effet de Toggle
          (`self.Set_Game_Speed` _output_get) ; On définie le nouveau Game Speed à 1
          (bind _foundwidgets_2 (`WidgetBlueprintLibrary.GetAllWidgetsOfClass` "/Game/Totem/HUD/InGame_Widget/WBP_InGame.WBP_InGame_C"))
          (`/Game/Totem/HUD/InGame_Widget/WBP_Time_Control.Set_Game_Speed_From_Player_Controller` (`/Game/Totem/HUD/InGame_Widget/WBP_InGame.WBP_Time_Control` (`|GetArrayItem` _foundwidgets_2)) _output_get) ; On modifie WBP_Time_Control
        )))))

(event `InputAction|Mouse_Left_Click`
  (params (Key :type "Key Structure"))
  (bind _hitresult (`self.GetHitResultUnderCursorByChannel` "TraceTypeQuery1"))
  (bind _building_placing_link (`self.Building_Placing_Link`))
  ;[1 1 1] Left Click Interaction
  (:`Pressed`
    (if (`GameplayStatics.BreakHitResult` _hitresult)
      (set `self.Mouse_Hit_Actor` (`.HitActor` (`GameplayStatics.BreakHitResult` _hitresult)))
      (if (`KismetSystemLibrary.DoesImplementInterface` (`.HitActor` (`GameplayStatics.BreakHitResult` _hitresult)) "/Game/Totem/Utilities/Interfaces/BP_Interface_Clickable.BP_Interface_Clickable_C")
        (if (`self.Is_Placing_New_Item?`)
          (message `/Game/Totem/Utilities/Interfaces/BP_Interface_Clickable.Place_New_Item` (`self.Mouse_Hit_Actor`))
          (elif (`self.Placing_Link?`)
            (bind _asbp_interactable (cast `/Game/Totem/Actors/Interactable/BP_Interactable` (`self.Mouse_Hit_Actor`)))
            (if (`/Game/Totem/Actors/Interactable/Buildings/BP_Buildings.Linkable?` _building_placing_link)
              (`/Game/Totem/Actors/Interactable/Buildings/BP_Buildings.Create_Link` _building_placing_link _asbp_interactable))
            (else
              (bind _asbp_interactable_2 (cast `/Game/Totem/Actors/Interactable/BP_Interactable` (`self.Mouse_Hit_Actor`) :!label _label_4)
                (:`then`
                  (message `/Game/Totem/Utilities/Interfaces/BP_Interface_Clickable.Interact` _asbp_interactable_2))
                (:`CastFailed`
                  (bind _outactors (`GameplayStatics.GetAllActorsOfClass` "/Game/Totem/Actors/Interactable/BP_Interactable.BP_Interactable_C" :!label _label_5))
                  (for _array_element _outactors
                    (`SceneComponent.SetVisibility` (`/Game/Totem/Actors/Interactable/BP_Interactable.Assignation_Widget` _array_element) false false)
                    (`/Game/Totem/Actors/Interactable/BP_Interactable.Unselected_Outline` _array_element)))))))
        (else
          (goto _label_4)))
      (else
        (goto _label_5)))))

(event `Game_Speed_Event`
  (params (Speed :type Integer))
  ;[1 1 1] Start Stop Game
  (`self.Set_Game_Speed` Speed) ; On définie le nouveau Game Speed
  (bind _foundwidgets (`WidgetBlueprintLibrary.GetAllWidgetsOfClass` "/Game/Totem/HUD/InGame_Widget/WBP_InGame.WBP_InGame_C"))
  (`/Game/Totem/HUD/InGame_Widget/WBP_Time_Control.Set_Game_Speed_From_Player_Controller` (`/Game/Totem/HUD/InGame_Widget/WBP_InGame.WBP_Time_Control` (`|GetArrayItem` _foundwidgets)) Speed) ; On modifie WBP_Time_Control
  (set `self.Current_Game_Speed` Speed))

(fn `Set_Game_Speed`
  (params (Speed :type Integer))
  (bind _outactors (`GameplayStatics.GetAllActorsOfClass` "/Script/Engine.Actor"))
  (for _array_element _outactors
    (if (and (!= _array_element (`/Game/Totem/Utilities/Function_Lib/Totem_Function_Library.Cast_Camera_Player`)) (!= _array_element (`/Game/Totem/Utilities/Function_Lib/Totem_Function_Library.Cast_BP_Player_Controller`)))
      (set `Actor.CustomTimeDilation` (`KismetMathLibrary.Conv_IntToDouble` Speed) _array_element))))

(fn `Set_Player_Max_Speed`
  (set `FloatingPawnMovement.MaxSpeed` (`KismetMathLibrary.FClamp` (- (`self.Player_Max_Speed`) (`KismetMathLibrary.Conv_IntToDouble` (* (`self.Zoom_Level`) 500))) 3000.0 8000.0) (`/Game/Totem/Actors/Player/BP_Camera_Player.FloatingPawnMovement` (`/Game/Totem/Utilities/Function_Lib/Totem_Function_Library.Cast_Camera_Player`))))

(fn `UserConstructionScript`)