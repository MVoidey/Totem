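; Map tile actor that hosts a village building slot, moves the item being placed onto itself on hover, and can be corrupted.
; A widget button shows on buildable tiles; building creation spawns the game mode's class for its BuildingType and unlocks nearby tiles with the next village index.
; Corruption switches the material, plays a randomly tilted fall timeline, then destroys the tile and attached actors.
; Random foliage scattering exists but never runs.
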(event `self.ReceiveBeginPlay`
  (bind _returnvalue (`KismetMathLibrary.RandomFloatInRange` -50.0 50.0))
  (`|ExecutionSequence`
    (:`then_0`
      (bind _returnvalue_2 (`PrimitiveComponent.CreateDynamicMaterialInstance` (`self.Tuile`) 0 "/Game/Totem/Material/Tuile/Tile_Mat.Tile_Mat" "None"))
      (set `self.Tile_Mat` _returnvalue_2)
      (set `self.X_Rot` _returnvalue)
      (set `self.Y_Rot` _returnvalue))
    (:`then_1`
      (bind _aswbp_map_tile_building (cast `/Game/Totem/HUD/Construction_Widget/WBP_Map_Tile_Building` (`WidgetComponent.GetWidget` (`self.Building_Button`))))
      (set `/Game/Totem/HUD/Construction_Widget/WBP_Map_Tile_Building.Building Type` (`self.Building_Type`) _aswbp_map_tile_building)
      (set `/Game/Totem/HUD/Construction_Widget/WBP_Map_Tile_Building.Village_Creation_Index` (`self.Village_Creation_Index`) _aswbp_map_tile_building)
      (add `/Game/Totem/HUD/Basic_Widget/WBP_Basic_Button.OnClicked` (`/Game/Totem/HUD/Construction_Widget/WBP_Map_Tile_Building.WBP_Basic_Button` _aswbp_map_tile_building) (`|CreateDelegate` :!event `ED_Create_Building`)))
    (:`then_2`
      (if (== (`self.Village_Creation_Index`) 1)
        (set `self.Buildable?` true)))))

(event `self.ReceiveActorBeginCursorOver`
  (bind _returnvalue (`GameplayStatics.GetActorOfClass` "/Game/Totem/Actors/New_Item/BP_New_Item.BP_New_Item_C"))
  (`/Engine/EditorBlueprintResources/StandardMacros.IsValid` _returnvalue
    (:`Is Valid`
      (`/Game/Totem/Actors/New_Item/BP_New_Item.Set_New_Location` _returnvalue (`self.K2_GetActorLocation`)))))

(event `/Game/Totem/Utilities/Interfaces/BP_Interface_Clickable.Place_New_Item`
  (bind _returnvalue (`GameplayStatics.GetActorOfClass` "/Game/Totem/Actors/New_Item/BP_New_Item.BP_New_Item_C"))
  (message `/Game/Totem/Utilities/Interfaces/BP_Interface_Clickable.Place_New_Item` _returnvalue))

(event `Corrupted`
  (`MaterialInstanceDynamic.SetScalarParameterValue` (`self.Tile_Mat`) "Switch" 1.0) ; Change la couleur de la tuile
  (bind (_direction _translate_z _rotation) (`Timeline|Falling` :!via `PlayFromStart`) ; Déclenche l'animation de chute
    (:`Update`
      (`self.K2_SetActorRelativeLocation` (`KismetMathLibrary.MakeVector` 0.0 0.0 _translate_z))
      (`self.K2_SetActorRelativeRotation` (`KismetMathLibrary.MakeRotator` (`KismetMathLibrary.Lerp` 0.0 (`self.X_Rot`) _rotation) (`KismetMathLibrary.Lerp` 0.0 (`self.Y_Rot`) _rotation))))
    (:`Finished`
      (`KismetSystemLibrary.Delay` 0.1) ; Une fois l'animation terminé, détruit\nl'acteur
      (for _array_element (`self.GetAttachedActors` true)
        (`self.K2_DestroyActor` _array_element))
      (`KismetSystemLibrary.Delay` 0.1)
      (`self.K2_DestroyActor`))))

(fn `Destroy_Widget`
  (`ActorComponent.K2_DestroyComponent` (`self.Building_Button`)))

(fn `ED_Create_Building`
  (`|ExecutionSequence`
    (:`then_0`
      (`|SpawnActorFromClass` (`.Actor_Class_39_3261200A47C10D1B9017B6B8D33FBB90` (break `/Game/Totem/Utilities/Structure/Building_Structure` (`BlueprintMapLibrary.Map_Find` (`/Game/Totem/Actors/GameMode/BP_Main_GameMode.Building_Rules` (`/Game/Totem/Utilities/Function_Lib/Totem_Function_Library.Cast_GameMode`)) (`self.Building_Type`)))) (`KismetMathLibrary.MakeTransform` (`self.K2_GetActorLocation`)) "Undefined" "OverrideRootScale" null null)
      (`ActorComponent.K2_DestroyComponent` (`self.Building_Button`))
      (`self.Update_Neighbour_Buildibility`))
    (:`then_1`
      (bind _foundwidgets (`WidgetBlueprintLibrary.GetAllWidgetsOfClass` "/Game/Totem/HUD/InGame_Widget/WBP_Game_Widget.WBP_Game_Widget_C"))
      (bind _wbp_village_construction (`/Game/Totem/HUD/InGame_Widget/WBP_Game_Widget.WBP_Village_Construction` (`|GetArrayItem` _foundwidgets)))
      (set `/Game/Totem/HUD/Construction_Widget/WBP_Village_Construction.Menu_Open?` false _wbp_village_construction)
      (remove `/Game/Totem/HUD/Construction_Widget/WBP_Village_Construction.Show_Village_Buildings` _wbp_village_construction (`|CreateDelegate` :!event `ED_Show_Building_Button`))
      (remove `/Game/Totem/HUD/Construction_Widget/WBP_Village_Construction.Hide_Village_Buildings` _wbp_village_construction (`|CreateDelegate` :!event `ED_Hide_Building_Button`))
      (`/Game/Totem/HUD/Construction_Widget/WBP_Village_Construction.Hide_Village_Buildings` _wbp_village_construction))))

(fn `ED_Hide_Building_Button`
  (`SceneComponent.SetVisibility` (`self.Building_Button`) false false))

(fn `ED_Show_Building_Button`
  (if (`self.Buildable?`)
    (`SceneComponent.SetVisibility` (`self.Building_Button`) true false)))

(fn `Update_Neighbour_Buildibility`
  (bind _outactors (`GameplayStatics.GetAllActorsOfClass` "BP_Map_Tile_C"))
  (for _array_element _outactors
    (if (< (`KismetMathLibrary.Vector_Distance` (`self.K2_GetActorLocation` _array_element) (`self.K2_GetActorLocation`)) 1800.0)
      (if (not (`/Game/Totem/Actors/Tile/BP_Map_Tile.Buildable?` _array_element))
        (set `/Game/Totem/Actors/Tile/BP_Map_Tile.Buildable?` true _array_element)
        (set `/Game/Totem/Actors/Tile/BP_Map_Tile.Village_Creation_Index` (+ (`self.Village_Creation_Index`) 1) _array_element)))))

(fn `UserConstructionScript`)