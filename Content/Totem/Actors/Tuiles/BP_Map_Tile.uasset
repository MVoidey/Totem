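; Map tile actor that serves as a mouse-driven target for placing buildings.
; It caches BP_Player on BeginPlay and sends it the tile's location as the new item position on cursor hover.
; A click clears the player's placing flag and calls Spawn on the pending BP_Buildings_Actor, without checking that flag first.
; The construction script is empty; its randomized radial grass and mushroom scattering is disconnected, as is an older resource-placement branch.
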(event `self.ReceiveBeginPlay`
  (bind _asbp_player (cast `/Game/Totem/Actors/Player/BP_Player` (`GameplayStatics.GetPlayerCharacter` 0)))
  (set `self.Player` _asbp_player))

(event `self.ReceiveActorBeginCursorOver`
  (`/Game/Totem/Actors/Player/BP_Player.Set_New_Item_Location` (`self.Player`) (`self.K2_GetActorLocation`)))

(event `self.ReceiveActorOnClicked`
  (params (ButtonPressed :type "Key Structure"))
  (bind _player (`self.Player`))
  (set `/Game/Totem/Actors/Player/BP_Player.Is_Placing_New_Item?` false _player)
  (bind _asbp_buildings_actor (cast `/Game/Totem/Actors/Interactable/Buildings/BP_Buildings_Actor` (`/Game/Totem/Actors/Player/BP_Player.New_Item_Actor` _player)))
  (`/Game/Totem/Actors/Interactable/Buildings/BP_Buildings_Actor.Spawn` _asbp_buildings_actor))

(fn `UserConstructionScript`)