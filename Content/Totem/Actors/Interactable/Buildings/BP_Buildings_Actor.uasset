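; Building actor in the Totem game with a spline meant to connect it to the nearest BP_Koro or other building.
; Create_Spline_Connexion starts from the Koro distance and compares all buildings, but appears unfinished: closer matches zero the variables instead of storing them.
; It then moves the first spline point to its own location, not the closest actor's.
; Spawn separately sets the second point and both tangents to fixed world-space values.
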(event `Create_Spline_Connexion`
  (`|ExecutionSequence`
    (:`then_0`
      ;[1 1 1] Cherche distance avec Koro et enregistre dans une variable
      (bind _returnvalue (`GameplayStatics.GetActorOfClass` "/Game/Totem/Actors/Interactable/Koro/BP_Koro.BP_Koro_C"))
      (bind _output_get (set `self.Closest_Distance` (`self.GetDistanceTo` _returnvalue self)))
      (set `self.Closest_Actor` _output_get))
    (:`then_1`
      ;[1 1 1] Vérirfie la distance avec les actors BP_Building
      (bind _outactors (`GameplayStatics.GetAllActorsOfClass` "BP_Buildings_Actor_C"))
      (for _array_element _outactors
        ;[1 1 1] Si la nouvelle distance est plus courte que la variable, la nouvelle distance devient la variable
        (if (< (`self.GetDistanceTo` _array_element self) (`self.Closest_Distance`))
          (set `self.Closest_Distance` 0.0)
          (set `self.Closest_Actor` 0.0)))
      ;[1 1 1] Place le dernier point de la spline sur la position de l'acteur le plus proche
      (`SplineComponent.SetLocationAtSplinePoint` (`self.Spline`) 0 (`self.K2_GetActorLocation`) "World" true))))

(event `Spawn`
  (bind _spline (`self.Spline`))
  (`SplineComponent.SetLocationAtSplinePoint` _spline 1 (0.0 0.0 200.0) "World" true)
  (`SplineComponent.SetTangentAtSplinePoint` _spline 0 (1000.0 1000.0 0.0) "World" true)
  (`SplineComponent.SetTangentAtSplinePoint` _spline 1 (1000.0 1000.0 0.0) "World" true))

(fn `UserConstructionScript`)