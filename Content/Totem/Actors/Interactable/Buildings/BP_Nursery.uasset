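; BP_Nursery is an interactable building that produces new villagers from a pending creation count.
; A DoOnce-gated timeline drives the creation percent, then decrements the count, spawns a BP_Villager at the nursery and re-triggers itself to work through the remaining queue.
; Each new villager is registered and assigned to the first non-full BP_House found in the level.
; BeginPlay sets the building type and the meshes to outline.
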(event `self.ReceiveBeginPlay`
  (set `self.Building_type` "NewEnumerator1")
  (`parent.ReceiveBeginPlay`)
  ;[1 1 1] Set Mesh to Outline
  (set `self.Meshes_to_Outline` (`|MakeArray` (`self.Nursery`) (`self.Roof`) :!type "PrimitiveComponent Object Reference")))

(event `Create_Villager`
  (if (> (`self.Villager_Creation_Amount`) 0)
    (`/Engine/EditorBlueprintResources/StandardMacros.DoOnce` false :!label _label
      (:`Completed`
        (bind (_direction _percent) (`Timeline|Villager_Creation_Timeline` :!via `PlayFromStart`)
          (:`Update`
            (set `self.Villager_Creation_Percent` _percent))
          (:`Finished`
            (`|ExecutionSequence`
              (:`then_0`
                (`/Engine/EditorBlueprintResources/StandardMacros.DecrementInt` (`self.Villager_Creation_Amount`)
                  (:`  `
                    (set `self.Villager_Creation_Percent` 0.0))))
              (:`then_1`
                (bind _returnvalue (`|SpawnActorFromClass` "/Game/Totem/Actors/Villager/BP_Villager.BP_Villager_C" (`KismetMathLibrary.MakeTransform` (`self.K2_GetActorLocation`)) "Undefined" "OverrideRootScale" null null))
                (`/Game/Totem/Utilities/Function_Lib/Totem_Function_Library.Add_Villager` _returnvalue)
                (`self.Assign_Villager_To_House` _returnvalue))
              (:`then_2`
                (goto _label :!via `Reset`))
              (:`then_3`
                (`self.Create_Villager`)))))))))

(event `Assign_Villager_To_House`
  (params (Villager :type "/Game/Totem/Actors/Villager/BP_Villager Object Reference (by ref)"))
  (bind _outactors (`GameplayStatics.GetAllActorsOfClass` "/Game/Totem/Actors/Interactable/Buildings/BP_House.BP_House_C"))
  (for _array_element _outactors
    (if (not (`/Game/Totem/Actors/Interactable/Buildings/BP_House.Full` _array_element))
      (set `self.House_to_Feed` _array_element)
      (break)))
  (`/Game/Totem/Actors/Interactable/Buildings/BP_House.Add_New_Villager` (`self.House_to_Feed`) Villager))

(fn `UserConstructionScript`
  (`parent.UserConstructionScript`))