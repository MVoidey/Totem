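; BP_House is a house building that raises the villager population cap and houses villagers.
; On BeginPlay it sets its building type, runs the parent logic, registers the house mesh and roof for outlining, and updates the game mode's villager maximum.
; Adding a villager puts it in the worker list, assigns the house through the villager's AI controller and flags the house full at capacity.
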(event `self.ReceiveBeginPlay`
  (set `self.Building_type` "NewEnumerator0")
  (`parent.ReceiveBeginPlay`)
  (`|ExecutionSequence`
    (:`then_0`
      ;[1 1 1] Set Mesh to Outline
      (set `self.Meshes_to_Outline` (`|MakeArray` (`self.House_Mesh`) (`self.Roof`) :!type "PrimitiveComponent Object Reference")))
    (:`then_1`
      (`self.Add_Max_Villager`))))

(event `Add_Max_Villager`
  (`/Engine/EditorBlueprintResources/StandardMacros.IncrementInt` (`.Max_7_CC1B05584084C96C3EA2DD908A3A51A9` (break `/Game/Totem/Utilities/Structure/Villager_Structure` (`/Game/Totem/Actors/GameMode/BP_Main_GameMode.Villager_Rules` (`/Game/Totem/Utilities/Function_Lib/Totem_Function_Library.Cast_GameMode`)))) (`self.Capacity`)))

(event `Add_New_Villager`
  (params (Villager :type "/Game/Totem/Actors/Villager/BP_Villager Object Reference (by ref)"))
  (`KismetArrayLibrary.Array_Add` (`self.Worker_List`) Villager)
  (bind _asbp_villager_ai_controller (cast `/Game/Totem/Actors/Villager/BP_Villager_AI_Controller` (`AIBlueprintHelperLibrary.GetAIController` Villager)))
  (`/Game/Totem/Actors/Villager/BP_Villager_AI_Controller.Set_House` _asbp_villager_ai_controller self)
  (if (>= (`KismetArrayLibrary.Array_Length` (`self.Worker_List`)) (`self.Capacity`))
    (set `self.Full` true)))

(fn `UserConstructionScript`
  (`parent.UserConstructionScript`))