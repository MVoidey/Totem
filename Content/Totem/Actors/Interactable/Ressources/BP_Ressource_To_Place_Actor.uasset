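; BP_Ressource_To_Place_Actor is a clickable resource placement marker in the Totem game.
; On BeginPlay it creates a dynamic material instance on its mesh, tints it with its Color variable, and caches the BP_Player character.
; When clicked, it passes its own location to the player's PlaceNewRessource, leaving the placement itself to the player.
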(event `self.ReceiveBeginPlay`
  (bind _returnvalue (`PrimitiveComponent.CreateDynamicMaterialInstance` (`self.Ressource_Mesh`) 0 "/Game/Totem/Material/Ressources/Ressource_To_Place_Mat.Ressource_To_Place_Mat" "None"))
  (`MaterialInstanceDynamic.SetVectorParameterValue` _returnvalue "Color" (`self.Color`))
  (bind _asbp_player (cast `/Game/Totem/Actors/Player/BP_Player` (`GameplayStatics.GetPlayerCharacter` 0)))
  (set `self.Player` _asbp_player))

(event `self.ReceiveActorOnClicked`
  (params (ButtonPressed :type "Key Structure"))
  (`/Game/Totem/Actors/Player/BP_Player.Place_New_Ressource` (`self.Player`) (`self.K2_GetActorLocation`)))

(fn `UserConstructionScript`)