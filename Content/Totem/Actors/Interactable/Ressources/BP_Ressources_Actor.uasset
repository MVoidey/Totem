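; Resource tile actor that villagers are assigned to harvest, with toggleable resource and full-stock widgets bound to it.
; Interacting toggles its resource widget, hiding those of all other resource actors.
; Adding or removing villagers moves them between the GameMode's available pool and CurrentWorker, directing their AI controllers to one of five work locations or stopping them.
; Destroy_When_Empty stops all workers and increments the available count before destroying the actor.
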(event `self.ReceiveBeginPlay`
  (`parent.ReceiveBeginPlay`)
  (`|ExecutionSequence`
    (:`then_0`
      (`self.Set_Type` "NewEnumerator0")
      (`self.Set_Widget`))
    (:`then_1`
      (set `self.Villager_Work_Locations` (`|MakeArray` (`self.Villager_Location_1`) (`self.Villager_Location_2`) (`self.Villager_Location_3`) (`self.Villager_Location_4`) (`self.Villager_Location_5`))))))

(event `Set_Widget`
  (`|ExecutionSequence`
    (:`then_0`
      (bind _aswbp_ressource_widget (cast `/Game/Totem/HUD/Ressources_Widget/WBP_Ressource_Widget` (`WidgetComponent.GetWidget` (`self.Ressource_Widget`))))
      (`/Game/Totem/HUD/Ressources_Widget/WBP_Ressource_Widget.Set_Owner` _aswbp_ressource_widget self))
    (:`then_1`
      (bind _aswbp_full_stock_widget (cast `/Game/Totem/HUD/Ressources_Widget/WBP_Full_Stock_Widget` (`WidgetComponent.GetWidget` (`self.Full_Stock_Widget`))))
      (`/Game/Totem/HUD/Ressources_Widget/WBP_Full_Stock_Widget.Set_Owner` _aswbp_full_stock_widget self))))

(event `Set_Type`
  (params (Tile_Type :type "/Game/Totem/Utilities/Enum/Ressource_Type Enum" :default "NewEnumerator0"))
  (set `self.Tile_Type` Tile_Type))

(event `/Game/Totem/Actors/Player/BP_Interface_Clickable.Interact`
  ;[1 1 1] On Clicked Event pour afficher le Ressource_Widget
  (if (`SceneComponent.bVisible` (`self.Ressource_Widget`))
    (`SceneComponent.SetVisibility` (`self.Ressource_Widget`) false false)
    (else
      (bind _outactors (`GameplayStatics.GetAllActorsOfClass` "BP_Ressources_Actor_C"))
      (for _array_element _outactors
        (`SceneComponent.SetVisibility` (`/Game/Totem/Actors/Interactable/Ressources/BP_Ressources_Actor.Ressource_Widget` _array_element) false false))
      (`SceneComponent.SetVisibility` (`self.Ressource_Widget`) true false))))

(event `Add_Villager`
  (bind (_villager_structure_amount _villager_structure_max _villager_structure_available _villager_structure_list) (break `/Game/Totem/Utilities/Structure/Villager_Structure` (`/Game/Totem/Actors/GameMode/BP_Main_GameMode.Villager_Structure` (`/Game/Totem/Utilities/Function_Lib/Totem_Function_Library.Cast_GameMode`))))
  (bind _output (`|GetArrayItem` _villager_structure_list (- _villager_structure_available 1)))
  ;[1 1 1] Ajouter un villageois
  (if (< (`self.Villager_Amount`) (`self.Max_Villager`))
    (if (> _villager_structure_available 0)
      (`/Engine/EditorBlueprintResources/StandardMacros.IncrementInt` (`self.Villager_Amount`)
        (:`  `
          (`KismetArrayLibrary.Array_AddUnique` (`self.Current_Worker`) _output) ; Ajoute à la liste des worker de la ressource
          (bind _asbp_villager_ai_controller (cast `/Game/Totem/Actors/Villager/BP_Villager_AI_Controller` (`AIBlueprintHelperLibrary.GetAIController` _output)))
          (`/Game/Totem/Actors/Villager/BP_Villager_AI_Controller.Assigned` _asbp_villager_ai_controller (`SceneComponent.K2_GetComponentLocation` (`|GetArrayItem` (`self.Villager_Work_Locations`) (- (`self.Villager_Amount`) 1))) self) ; Envoie l'IA récolter la ressource
          (`KismetArrayLibrary.Array_RemoveItem` _villager_structure_list _output)
          (`/Engine/EditorBlueprintResources/StandardMacros.DecrementInt` _villager_structure_available))))))

(event `Remove_Villager`
  (bind _current_worker (`self.Current_Worker`))
  (bind (_villager_structure_amount _villager_structure_max _villager_structure_available _villager_structure_list) (break `/Game/Totem/Utilities/Structure/Villager_Structure` (`/Game/Totem/Actors/GameMode/BP_Main_GameMode.Villager_Structure` (`/Game/Totem/Utilities/Function_Lib/Totem_Function_Library.Cast_GameMode`))))
  (bind _output (`|GetArrayItem` _current_worker (`KismetArrayLibrary.Array_LastIndex` _current_worker)))
  ;[1 1 1] Retirer un villageois
  (if (> (`self.Villager_Amount`) 0)
    (`/Engine/EditorBlueprintResources/StandardMacros.DecrementInt` (`self.Villager_Amount`)
      (:`  `
        (`/Engine/EditorBlueprintResources/StandardMacros.IncrementInt` _villager_structure_available
          (:`  `
            (`KismetArrayLibrary.Array_AddUnique` _villager_structure_list _output)
            (bind _asbp_villager_ai_controller (cast `/Game/Totem/Actors/Villager/BP_Villager_AI_Controller` (`AIBlueprintHelperLibrary.GetAIController` _output)))
            (`/Game/Totem/Actors/Villager/BP_Villager_AI_Controller.Stop_Getting_Ressources` _asbp_villager_ai_controller)
            (`KismetArrayLibrary.Array_RemoveItem` (`self.Current_Worker`) _output) ; Retire de la liste des worker
          ))))))

(event `Destroy_When_Empty`
  (bind (_villager_structure_amount _villager_structure_max _villager_structure_available) (break `/Game/Totem/Utilities/Structure/Villager_Structure` (`/Game/Totem/Actors/GameMode/BP_Main_GameMode.Villager_Structure` (`/Game/Totem/Utilities/Function_Lib/Totem_Function_Library.Cast_GameMode`))))
  ;[1 1 1] Détruit l'acteur quand il est vide
  (for _array_element (`self.Current_Worker`)
    (bind _asbp_villager_ai_controller (cast `/Game/Totem/Actors/Villager/BP_Villager_AI_Controller` (`AIBlueprintHelperLibrary.GetAIController` _array_element)))
    (`/Game/Totem/Actors/Villager/BP_Villager_AI_Controller.Stop_Getting_Ressources` _asbp_villager_ai_controller)
    (`/Engine/EditorBlueprintResources/StandardMacros.IncrementInt` _villager_structure_available))
  (`self.K2_DestroyActor`))

(fn `UserConstructionScript`)