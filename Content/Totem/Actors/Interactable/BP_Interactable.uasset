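; BP_Interactable is an interactable actor that sits on a map tile and shows an outline when hovered or selected.
; On BeginPlay it searches all BP_Map_Tile actors and attaches itself, keeping world transform, to any sharing its exact X and Y location.
; Cursor and selection events toggle Render Custom Depth on MeshesToOutline, with a Selected flag keeping the outline on after the cursor leaves.
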(event `self.ReceiveBeginPlay`
  (bind (_returnvalue_x _returnvalue_y) (`KismetMathLibrary.BreakVector` (`self.K2_GetActorLocation`)))
  (bind _outactors (`GameplayStatics.GetAllActorsOfClass` "/Game/Totem/Actors/Tuiles/BP_Map_Tile.BP_Map_Tile_C"))
  (for _array_element _outactors
    (bind (_returnvalue_x_2 _returnvalue_y_2) (`KismetMathLibrary.BreakVector` (`self.K2_GetActorLocation` _array_element)))
    (if (and (== _returnvalue_x_2 _returnvalue_x) (== _returnvalue_y_2 _returnvalue_y))
      (`self.K2_AttachToActor` _array_element "None" "KeepWorld" "KeepWorld" "KeepWorld"))))

(event `self.ReceiveActorBeginCursorOver`
  ;[1 1 1] Outline On/Off Event
  (for _array_element (`self.Meshes_to_Outline`) :!label _label
    (`PrimitiveComponent.SetRenderCustomDepth` _array_element true)))

(event `Selected_Outline`
  ;[1 1 1] Outline On/Off Event
  (set `self.Selected?` true)
  (goto _label))

(event `self.ReceiveActorEndCursorOver`
  ;[1 1 1] Outline On/Off Event
  (if (not (`self.Selected?`))
    (for _array_element (`self.Meshes_to_Outline`) :!label _label_2
      (`PrimitiveComponent.SetRenderCustomDepth` _array_element false))))

(event `Unselected_Outline`
  ;[1 1 1] Outline On/Off Event
  (set `self.Selected?` false)
  (goto _label_2))

(fn `UserConstructionScript`)