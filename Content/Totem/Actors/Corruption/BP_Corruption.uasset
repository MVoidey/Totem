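; BP_Corruption is the actor that drives corruption spreading inward across the map tiles toward the Koro.
; On BeginPlay it maps every BP_Map_Tile to its distance from a fixed Koro position and uses the farthest as the radius.
; Corruption_Randomness rolls a percentage chance, either shrinking the radius with a camera shake or raising the next chance.
; Growing corrupts and unregisters tiles outside the radius through a delayed loop.
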(event `self.ReceiveBeginPlay`
  (`|ExecutionSequence`
    (:`then_0`
      ;[1 1 1] Création du radius de la corruption
      (bind _outactors (`GameplayStatics.GetAllActorsOfClass` "/Game/Totem/Actors/Tuiles/BP_Map_Tile.BP_Map_Tile_C"))
      (for _array_element _outactors
        (`BlueprintMapLibrary.Map_Add` (`self.Map_Tiles_Distance`) _array_element (`KismetMathLibrary.Vector_Distance` (0.0 0.0 200.0) (`self.K2_GetActorLocation` _array_element))) ; Crée une map avec chaque\ntuiles en key, et sa distance avec\nle Koro en value
      )
      (bind _values (`BlueprintMapLibrary.Map_Values` (`self.Map_Tiles_Distance`)))
      (set `self.Radius` (`.MaxValue` (`KismetMathLibrary.MaxOfFloatArray` _values))) ; Et devient le radius de la corruption
    )))

(event `Growing`
  (bind _map_tiles_distance (`self.Map_Tiles_Distance`))
  ;[1 1 1] La corruption grandit
  (set `self.Radius` (- (`self.Radius`) (`self.Radius_Reducer`))) ; Réduit la taille du radius
  (bind _keys (`BlueprintMapLibrary.Map_Keys` _map_tiles_distance))
  (bind _array_element (`/Game/Totem/Utilities/Macro_Lib/BP_Custom_Macro.For_Each_Loop_With_Delay` _keys 0.005)
    (:`Loop_Body`
      (if (> (`BlueprintMapLibrary.Map_Find` _map_tiles_distance _array_element) (`self.Radius`))
        (`/Game/Totem/Actors/Tuiles/BP_Map_Tile.Corrupted` _array_element)
        (`BlueprintMapLibrary.Map_Remove` (`self.Map_Tiles_Distance`) _array_element)))))

(event `Corruption_Randomness`
  ;[1 1 1] Lancé de dé de la corruption
  (bind _output_get (set `self.Picked_Chance` (`KismetMathLibrary.RandomIntegerInRange` 0 100)))
  (if (<= _output_get (`self.Corruption_Chance`))
    (`self.Growing`) ; Si oui, la corruption grandit
    (`PlayerController.ClientStartCameraShake` :`self` (`/Game/Totem/Utilities/Function_Lib/Totem_Function_Library.Cast_BP_Player_Controller`) :`Shake` "/Game/Totem/Actors/Player/BP_Camera_Shake.BP_Camera_Shake_C") ; Lance une animation de CamShake
    (else
      (`/Engine/EditorBlueprintResources/StandardMacros.IncrementInt` (`self.Corruption_Chance`) 5) ; Si non, ajout 5% de chance
    )))

(fn `UserConstructionScript`)