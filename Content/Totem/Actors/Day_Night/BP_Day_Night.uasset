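; Day/night cycle actor that drives the sun, sky and clock, and starts and ends the villagers' workday.
; A 60-second timeline, scaled by PlayRate, animates sun rotation and intensity, global light color, a dynamic sky material and the HUD clock.
; Its Start/End Day events toggle lights through BP_Interface_Lighting and make villager controllers gather or consume resources, staggered by delayed loops.
; Day start also increments the GameMode's DayCount.
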(event `self.ReceiveBeginPlay`
  (`KismetSystemLibrary.Delay` 0.2)
  (`|ExecutionSequence`
    (:`then_0`
      (bind _returnvalue (`PrimitiveComponent.CreateDynamicMaterialInstance` (`self.SkySphere`) 0 "/Game/Totem/Material/SkySphere/SkySphere_Mat.SkySphere_Mat" "None")) ; Crée une material dynamique pour la SkySphere
      (set `self.SkySphere_Mat` _returnvalue))
    (:`then_1`
      (if (`self.Start_Day_Cycle`)
        (if (`self.Start_at_Sunrise`)
          (`self.StartGame_DayLight`))
        (`self.Light_Cycle`) ; Déclenche le cycle Jour Nuit
        (`TimelineComponent.SetPlayRate` (`self.DayLight_Cycle_TimeLine`) (`self.PlayRate`)) ; Change la vitesse de lecture de la Timeline
      ))))

(event `Light_Cycle`
  (bind (_direction _daylight_rotation _daylight_intensity _skysphere_gradient_offset _gradient_offset_2 _global_light_color _clock_needle_rotation) (`Timeline|DayLight_Cycle_TimeLine` :`NewTime` 10.0 :!label _label) ; Création d'une Timeline\nElle est construite sur une base de 60 sec\nOn pourra ralonger la durée des journée en modifiant \nle PlayRate
    (:`Update`
      (`|ExecutionSequence`
        (:`then_0`
          (`SceneComponent.K2_SetRelativeRotation` (`self.DayLight_Parent`) (`KismetMathLibrary.MakeRotator` _daylight_rotation) false false)
          (`LightComponent.SetIntensity` (`self.Day Light`) _daylight_intensity)
          (`MaterialInstanceDynamic.SetScalarParameterValue` (`self.SkySphere_Mat`) "Gradient_Offset" _skysphere_gradient_offset)
          (`MaterialInstanceDynamic.SetScalarParameterValue` (`self.SkySphere_Mat`) "Gradient_Offset2" _gradient_offset_2))
        (:`then_1`
          (`LightComponent.SetLightColor` (`self.GlobalLight`) _global_light_color true)
          (bind _foundwidgets (`WidgetBlueprintLibrary.GetAllWidgetsOfClass` "/Game/Totem/HUD/InGame_Widget/WBP_InGame.WBP_InGame_C"))
          (`/Game/Totem/HUD/InGame_Widget/WBP_DayClock.Set_Clock` (`/Game/Totem/HUD/InGame_Widget/WBP_InGame.WBP_DayClock` (`|GetArrayItem` _foundwidgets)) _clock_needle_rotation))))
    (:`Start_Day`
      (bind _outactors (`GameplayStatics.GetAllActorsWithInterface` "/Game/Totem/Utilities/Interfaces/BP_Interface_Lighting.BP_Interface_Lighting_C"))
      (for _array_element _outactors
        (message `/Game/Totem/Utilities/Interfaces/BP_Interface_Lighting.Deactivate_Light` _array_element))
      (`self.Start_Day`)
      (`/Engine/EditorBlueprintResources/StandardMacros.IncrementInt` (`/Game/Totem/Actors/GameMode/BP_Main_GameMode.Day_Count` (`/Game/Totem/Utilities/Function_Lib/Totem_Function_Library.Cast_GameMode`))))
    (:`End_Day`
      (bind _outactors_2 (`GameplayStatics.GetAllActorsWithInterface` "/Game/Totem/Utilities/Interfaces/BP_Interface_Lighting.BP_Interface_Lighting_C"))
      (for _array_element_2 _outactors_2
        (message `/Game/Totem/Utilities/Interfaces/BP_Interface_Lighting.Activate_Light` _array_element_2))
      (`self.End_Day`))))

(event `StartGame_DayLight`
  (goto _label :!via `SetNewTime`))

(event `Start_Day`
  (bind _outactors (`GameplayStatics.GetAllActorsOfClass` "/Game/Totem/Actors/Villager/BP_Villager_AI_Controller.BP_Villager_AI_Controller_C"))
  (bind _array_element (`/Game/Totem/Utilities/Macro_Lib/BP_Custom_Macro.For_Each_Loop_With_Delay` _outactors 0.2)
    (:`Loop_Body`
      (if (`/Game/Totem/Actors/Villager/BP_Villager_AI_Controller.Assigned?` _array_element)
        (`/Game/Totem/Actors/Villager/BP_Villager_AI_Controller.Start_Getting_Ressources` _array_element)))))

(event `End_Day`
  (bind _outactors (`GameplayStatics.GetAllActorsOfClass` "/Game/Totem/Actors/Villager/BP_Villager_AI_Controller.BP_Villager_AI_Controller_C"))
  (bind _array_element (`/Game/Totem/Utilities/Macro_Lib/BP_Custom_Macro.For_Each_Loop_With_Delay` _outactors 0.2)
    (:`Loop_Body`
      (`/Game/Totem/Actors/Villager/BP_Villager_AI_Controller.Stop_Getting_Ressources` _array_element)
      (`/Game/Totem/Actors/Villager/BP_Villager_AI_Controller.Use_Ressources` _array_element))))

(fn `UserConstructionScript`
  (`SceneComponent.SetWorldScale3D` (`self.SkySphere`) (`KismetMathLibrary.Conv_DoubleToVector` (`self.SkySphere_Size`)))
  (`SceneComponent.K2_SetWorldLocation` (`self.SkySphere`) (0.0 0.0 0.0) false false))