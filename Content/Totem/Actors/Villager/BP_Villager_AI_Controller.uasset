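; AI controller for villagers that switches behavior trees between waiting for assignment, construction work, resource gathering and eating.
; On begin play it starts the waiting tree and seeds the Blackboard with the Koro location and the game mode's work speed.
; Assignment writes a work slot location picked by villager count, plus resource type and an empty-out flag when already carrying resources.
; Workplace type selects the work tree on assignment and day start.
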(event `self.ReceiveBeginPlay`
  (`self.RunBehaviorTree` "/Game/Totem/Actors/Villager/Villager_AI_System/BTree_Villager_Waiting_Assignment.BTree_Villager_Waiting_Assignment")
  (`BlackboardComponent.SetValueAsVector` (`self.Blackboard`) "Koro_Location" (0.0 0.0 200.0))
  (`BlackboardComponent.SetValueAsFloat` (`self.Blackboard`) "Work_Speed" (`KismetMathLibrary.Conv_IntToDouble` (`.Work_Speed_17_4EF0279946E957ADEFF1C9ABA1F25832` (break `/Game/Totem/Utilities/Structure/Villager_Structure` (`/Game/Totem/Actors/GameMode/BP_Main_GameMode.Villager_Rules` (`/Game/Totem/Utilities/Function_Lib/Totem_Function_Library.Cast_GameMode`)))))))

(event `Assigned`
  (params (Workplace_Actor :type "/Game/Totem/Actors/Interactable/BP_Interactable Object Reference"))
  (bind _output_get (set `self.Workplace_Actor` Workplace_Actor))
  (`self.Workplace_Assignation`)
  (switch `/Game/Totem/Utilities/Enum/Interactable_Type` (`/Game/Totem/Actors/Interactable/BP_Interactable.Interactable_Type` _output_get)
    (:`NewEnumerator0`
      (`self.RunBehaviorTree` "/Game/Totem/Actors/Villager/Villager_AI_System/BTree_Villager_Construction_Assignation.BTree_Villager_Construction_Assignation"))
    (:`NewEnumerator1`
      (`self.RunBehaviorTree` "/Game/Totem/Actors/Villager/Villager_AI_System/BTree_Villager_Ressource_Assignation.BTree_Villager_Ressource_Assignation"))))

(event `Workplace_Assignation`
  (set `self.Assigned?` true)
  (bind _output_get (set `self.Ressource_Workplace_Location` (`SceneComponent.K2_GetComponentLocation` (`|GetArrayItem` (`/Game/Totem/Actors/Interactable/BP_Interactable.Villager_Work_Locations` (`self.Workplace_Actor`)) (- (`/Game/Totem/Actors/Interactable/BP_Interactable.Villager_Amount` (`self.Workplace_Actor`)) 1)))))
  (`BlackboardComponent.SetValueAsVector` (`self.Blackboard`) "Workplace_Location" _output_get) ; Définie la Workplace_Location du BlackBoard
  (switch `/Game/Totem/Utilities/Enum/Interactable_Type` (`/Game/Totem/Actors/Interactable/BP_Interactable.Interactable_Type` (`self.Workplace_Actor`))
    (:`NewEnumerator1`
      (bind _asbp_ressources_actor (cast `/Game/Totem/Actors/Interactable/Ressources/BP_Ressources_Actor` (`self.Workplace_Actor`)))
      (`BlackboardComponent.SetValueAsEnum` (`self.Blackboard`) "Ressource_Type" (`/Game/Totem/Actors/Interactable/Ressources/BP_Ressources_Actor.Tile_Type` _asbp_ressources_actor))
      (if (> (`BlackboardComponent.GetValueAsInt` (`self.Blackboard`) "Ressource_Amount") 0)
        (`BlackboardComponent.SetValueAsBool` (`self.Blackboard`) "Has_to_Become_Empty?" true)))))

(event `Remove_Assignation`
  (`self.RunBehaviorTree` "/Game/Totem/Actors/Villager/Villager_AI_System/BTree_Villager_Waiting_Assignment.BTree_Villager_Waiting_Assignment"))

(event `Start_Day`
  (switch `/Game/Totem/Utilities/Enum/Interactable_Type` (`/Game/Totem/Actors/Interactable/BP_Interactable.Interactable_Type` (`self.Workplace_Actor`))
    (:`NewEnumerator0`
      (`self.RunBehaviorTree` "/Game/Totem/Actors/Villager/Villager_AI_System/BTree_Villager_Construction_Assignation.BTree_Villager_Construction_Assignation"))
    (:`NewEnumerator1`
      (`self.RunBehaviorTree` "/Game/Totem/Actors/Villager/Villager_AI_System/BTree_Villager_Ressource_Assignation.BTree_Villager_Ressource_Assignation"))))

(event `Eat_Ressources`
  (`self.RunBehaviorTree` "/Game/Totem/Actors/Villager/Villager_AI_System/BTree_Villager_Eat_Ressources.BTree_Villager_Eat_Ressources"))

(fn `UserConstructionScript`)