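; BP_Villager is a villager actor whose point light reflects night time and whose time scale follows the game speed.
; On BeginPlay it sets its custom time dilation from the player controller's CurrentGameSpeed, then turns the light on if BP_Day_Night reports night.
; It also exposes events to show or hide the light and to destroy the actor, none of which poll for changes.
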(event `self.ReceiveBeginPlay`
  (`self.Set_Time_Dilation`)
  (bind _returnvalue (`GameplayStatics.GetActorOfClass` "/Game/Totem/Actors/Day_Night/BP_Day_Night.BP_Day_Night_C"))
  (if (`/Game/Totem/Actors/Day_Night/BP_Day_Night.Is_Night?` _returnvalue)
    (`self.Activate_Light`)))

(event `self.Activate_Light`
  (`SceneComponent.SetVisibility` (`self.PointLight`) true false))

(event `self.Deactivate_Light`
  (`SceneComponent.SetVisibility` (`self.PointLight`) false false))

(event `Destroy_Actor`
  (`self.K2_DestroyActor`))

(fn `Set_Time_Dilation`
  (set `self.CustomTimeDilation` (`KismetMathLibrary.Conv_IntToDouble` (`/Game/Totem/Actors/Player/BP_Player_Controller.Current_Game_Speed` (`/Game/Totem/Utilities/Function_Lib/Totem_Function_Library.Cast_BP_Player_Controller`)))))

(fn `UserConstructionScript`)