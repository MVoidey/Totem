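; Island generator actor that builds a tile map from child actor components, then spawns resources and BP_Koro on it.
; Construction script grows base rings around a center tile, then attaches seeded random tiles on free neighboring positions.
; At BeginPlay, it reads enabled resources and amounts from the game mode and spawns them on random-tile positions, removing neighbors to space them out.
; BP_Koro spawns at the center; the seed is randomized only while Reset is false.
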(event `self.ReceiveBeginPlay`
  (bind _ressources_setup (`/Game/Totem/Actors/GameMode/BP_Main_GameMode.Ressources_SetUp` (`/Game/Totem/Utilities/Function_Lib/Totem_Function_Library.Cast_GameMode`)))
  (`|ExecutionSequence`
    (:`then_0`
      ;[1 1 1] Set up de la repartition des ressources sur la map
      (bind _keys (`BlueprintMapLibrary.Map_Keys` _ressources_setup))
      (for _array_element _keys
        (bind (_onoff _spawn_amount _actor_class) (break `/Game/Totem/Utilities/Structure/Ressource_Structure` (`BlueprintMapLibrary.Map_Find` _ressources_setup _array_element)))
        (if _onoff
          (`BlueprintMapLibrary.Map_Add` (`self.BP_Ressources_Repartition`) _actor_class _spawn_amount))))
    (:`then_1`
      (`self.Spawn_Ressources_Actors`)
      (`self.Spawn_Koro`))))

(event `Spawn_Ressources_Actors`
  (bind _available_locations_for_ressources (`self.Available_Locations_for_Ressources`))
  ;[1 1 1] Création des BP_Ressources aléatoirement basé sur la seed
  (bind _keys (`BlueprintMapLibrary.Map_Keys` (`self.BP_Ressources_Repartition`)))
  (for _array_element _keys
    (for _ (range 1 (+ (`BlueprintMapLibrary.Map_Find` (`self.BP_Ressources_Repartition`) _array_element) 1))
      (bind _output_get (set `self.New_Ressource_Location` (`|GetArrayItem` _available_locations_for_ressources (`KismetMathLibrary.RandomIntegerInRangeFromStream` 0 (`KismetArrayLibrary.Array_LastIndex` _available_locations_for_ressources) (`self.Seed`)))))
      (`|SpawnActorFromClass` _array_element (`KismetMathLibrary.MakeTransform` (`KismetMathLibrary.MakeVector` (.x _output_get) (.y _output_get) 200.0)) "Undefined" "OverrideRootScale" null null) ; Crée l'acteur en fonction de la Key selectionné
      (`KismetArrayLibrary.Array_RemoveItem` (`self.Available_Locations_for_Ressources`) (`self.New_Ressource_Location`)) ; Retire la position de la nouvelle ressource\ndes positions disponibles
      (for _array_element_2 (`self.Close_Locations`)
        (`KismetArrayLibrary.Array_RemoveItem` (`self.Available_Locations_for_Ressources`) (+ _array_element_2 (`self.New_Ressource_Location`))) ; Retire toutes les positions autour de la\nnouvelle ressources créée, pour éviter\nque des ressources spawn trop proche
      )
      (`KismetArrayLibrary.Array_AddUnique` (`self.Occupied_Locations`) (`self.New_Ressource_Location`)) ; Ajoute la nouvelle position aux positions occupées
    )))

(event `Spawn_Koro`
  ;[1 1 1] Création du BP_Koro
  (`|SpawnActorFromClass` "/Game/Totem/Actors/Interactable/Koro/BP_Koro.BP_Koro_C" (`KismetMathLibrary.MakeTransform` (0.0 0.0 200.0)) "Undefined" "OverrideRootScale" null null)
  (`KismetArrayLibrary.Array_Add` (`self.Occupied_Locations`) (0.0 0.0 200.0)))

(fn `Add_Available_Location`
  ;[1 1 1] Pour toutes les positions autour de la tuile
  (for _array_element (`self.Close_Locations`)
    (bind _returnvalue (+ _array_element (`self.Last_Tile_Location`)))
    ;[1 1 1] Verifie que la position n'est pas déjà occupée
    (if (not (`KismetArrayLibrary.Array_Contains` (`self.Tile_Occupied_Locations`) _returnvalue))
      ;[1 1 1] Ajout la position à la liste des positions disponible
      (`KismetArrayLibrary.Array_AddUnique` (`self.Tile_Locations_Available`) _returnvalue))))

(fn `UserConstructionScript`
  (bind _tile_locations_available (`self.Tile_Locations_Available`))
  (if (not (`self.Reset`))
    (`KismetMathLibrary.SetRandomStreamSeed` (`self.Seed`) (`KismetMathLibrary.RandomInteger` 500))
    (set `self.Reset` true))
  (`|ExecutionSequence`
    (:`then_0`
      ;[1 1 1] Création première tuile
      (`AddComponent|NODE_AddChildActorComponent-10` :`RelativeTransform` (`KismetMathLibrary.MakeTransform` (0.0 0.0 200.0)))
      (`self.Add_Available_Location`))
    (:`then_1`
      ;[1 1 1] Création tuile du socle de base
      (for _ (range 1 (+ (`self.Base_Tile_Amount`) 1))
        (for _array_element (`self.Tile_Locations_Available`)
          (`AddComponent|NODE_AddChildActorComponent-14` :`RelativeTransform` (`KismetMathLibrary.MakeTransform` _array_element)))
        (`KismetArrayLibrary.Array_Append` (`self.Tile_Occupied_Locations`) (`self.Tile_Locations_Available`)) ; Les positions disponibles \ndeviennent occupées
        (`KismetArrayLibrary.Array_Clear` (`self.Tile_Locations_Available`)) ; Vide la liste des position disponible
        (for _array_element_2 (`self.Tile_Occupied_Locations`)
          (set `self.Last_Tile_Location` _array_element_2)
          (`self.Add_Available_Location`))))
    (:`then_2`
      ;[1 1 1] Création du reste de la carte avec des tuiles générées aléatoirement
      (for _ (range 1 (+ (`self.Random_Tile_Amount`) 1))
        (bind _output_get (set `self.Last_Tile_Location` (`|GetArrayItem` _tile_locations_available (`KismetMathLibrary.RandomIntegerInRangeFromStream` 0 (`KismetArrayLibrary.Array_LastIndex` _tile_locations_available) (`self.Seed`)))))
        (`AddComponent|NODE_AddChildActorComponent-13` :`RelativeTransform` (`KismetMathLibrary.MakeTransform` _output_get))
        (`KismetArrayLibrary.Array_RemoveItem` (`self.Tile_Locations_Available`) (`self.Last_Tile_Location`)) ; Retire la position choisie\ndes positions disponibles
        (`KismetArrayLibrary.Array_Add` (`self.Tile_Occupied_Locations`) (`self.Last_Tile_Location`)) ; Ajoute la position choisie\naux positions occupées
        (`self.Add_Available_Location`)
        (`KismetArrayLibrary.Array_Add` (`self.Available_Locations_for_Ressources`) (`self.Last_Tile_Location`))))))